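; BP_InspectActor displays a static mesh for inspection, with rotation by mouse drag.
; SetStaticMesh swaps the mesh, resets offset and rotation, then calls UpdateScale, which enlarges it uniformly toward DesiredExtent (never shrinking) and shifts it to center its bounds.
; Click start and end toggle rotation, while mouse-move deltas apply world yaw and pitch to the Scene component, turning the mesh.
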(fn `OnClickedEnd`
  (params (MouseLocation :type "Vector2D Structure"))
  (set `self.bRotationEnabled` false)
  (return))

(fn `OnClickedStart`
  (params (MouseLocation :type "Vector2D Structure"))
  (set `self.OnStartRotateLocation` MouseLocation)
  (set `self.bRotationEnabled` true)
  (return))

(fn `OnMouseMove`
  (params (MouseLocation :type "Vector2D Structure"))
  (bind (_x _y) (`KismetMathLibrary.BreakVector2D` (- MouseLocation (`self.OnStartRotateLocation`))))
  (if (`self.bRotationEnabled`)
    (`SceneComponent.K2_AddWorldRotation` (`self.Scene`) (`KismetMathLibrary.MakeRotator` 0.0 _y (* _x -1.0)) false false)
    (set `self.OnStartRotateLocation` (`local.MouseLocation`))
    (return)
    (else
      (return))))

(fn `SetStaticMesh`
  (params (NewMesh :type "StaticMesh Object Reference"))
  (`StaticMeshComponent.SetStaticMesh` (`self.StaticMesh`) NewMesh)
  (`SceneComponent.K2_SetRelativeLocation` (`self.StaticMesh`) (0.0 0.0 0.0) false false)
  (`SceneComponent.K2_SetRelativeRotation` :`self` (`self.Scene`))
  (`self.UpdateScale`))

(fn `UpdateScale`
  (locals (DesiredScale :type "Float (double-precision)" :default 0.0))
  (bind _staticmesh (`self.StaticMesh`))
  (bind _returnvalue (`KismetMathLibrary.GetMinElement` (/ (`self.DesiredExtent`) (`self.CurrentMeshExtent`))))
  (set `self.CurrentMeshExtent` (`.BoxExtent` (`KismetSystemLibrary.GetComponentBounds` (`self.StaticMesh`))))
  (if (< _returnvalue 1.0)
    (set `local.DesiredScale` 1.0)
    (else
      (set `local.DesiredScale` _returnvalue)))
  (`SceneComponent.SetWorldScale3D` (`self.StaticMesh`) (* (`SceneComponent.K2_GetComponentScale` (`self.StaticMesh`)) (`local.DesiredScale`)))
  (`SceneComponent.K2_AddLocalOffset` (`self.StaticMesh`) (- (`SceneComponent.K2_GetComponentLocation` _staticmesh) (`KismetSystemLibrary.GetComponentBounds` _staticmesh)) false true)
  (return))

(fn `UserConstructionScript`)