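; BP_Vase is an interactable world item that characters can pick up from or use inventory items on.
; Its Interact function switches on the action: Interact adds BaseItem to the BP_Character's inventory component.
; Use compares the class of the character's ItemUsing to BP_ItemRocketLauncher, removing it and returning true on a match, otherwise false, with debug prints.
; The event graph holds only disabled default events.
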(fn `Interact`
  (params (InstigatorPawn :type "Pawn Object Reference") (Action :type Name))
  (returns (ReturnValue :type Boolean))
  (bind _asbp_character (cast `/Game/JttU/Blueprints/Characters/BP_Character` InstigatorPawn :!pure true))
  (bind _itemusing (`JCharacter.ItemUsing` _asbp_character))
  (switch `name` Action
    (:`Interact`
      (`JInventoryComponent.AddItem` (`JCharacter.InventoryComponent` _asbp_character) (`self.BaseItem`)))
    (:`Use`
      (if (== (`GameplayStatics.GetObjectClass` _itemusing) "/Game/JttU/Blueprints/Data/Inventory/Items/BP_ItemRocketLauncher.BP_ItemRocketLauncher_C")
        (`JInventoryComponent.RemoveItem` (`JCharacter.GetInventoryComponent` _asbp_character) _itemusing)
        (`KismetSystemLibrary.PrintString` "PlayerItem Removed")
        (return true)
        (else
          (`KismetSystemLibrary.PrintString` "Player item not removed.")
          (return false))))))

(fn `UserConstructionScript`
  (`parent.UserConstructionScript`))