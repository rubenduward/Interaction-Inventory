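; BP_Lever is an interactable lever that toggles the lock on a linked actor.
; Interact flips its Enabled state and plays the matching on or off animation once on the skeletal mesh.
; If LinkedActor is valid, it inverts that actor's current Locked state via SetLock, independently of the lever's own state.
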(fn `Interact`
  (params (InstigatorPawn :type "Pawn Object Reference") (Action :type Name))
  (returns (ReturnValue :type Boolean))
  (locals (bOldEnabled :type Boolean :default false))
  (bind _linkedactor (`self.LinkedActor`))
  (bind _output_get (set `local.bOldEnabled` (`self.bEnabled`)))
  (`self.SetEnabled` (not _output_get))
  (`SkeletalMeshComponent.PlayAnimation` (`self.SkeletalMeshComp`) (select `bool` (`local.bOldEnabled`) :`false` (`self.AnimationOn`) :`true` (`self.AnimationOff`)) false)
  (`/Engine/EditorBlueprintResources/StandardMacros.IsValid` _linkedactor
    (:`Is Valid`
      (`JDoorActor.SetLock` _linkedactor (not (`JDoorActor.bLocked` _linkedactor)))
      (return false))))

(fn `UserConstructionScript`)