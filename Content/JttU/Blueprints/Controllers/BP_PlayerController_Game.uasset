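; Game player controller that links inventory input, the action menu for selected actors, and the controlled character.
; The Inventory action opens or closes the inventory widget through the game HUD.
; The actions widget receives the selected actor and appears at the cursor or at a usable actor's projected world location.
; Helpers start the character's move-to-usable timer, turn it yaw-only toward the selection, and expose its inspect actor.
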(event `InputAction|Inventory`
  (params (Key :type "Key Structure"))
  ;[1 1 1] Open/Close inventory
  (:`Pressed`
    (`self.ToggleInventory`)))

(fn `GetInspectActor`
  (returns (InspectActor :type "/Game/JttU/Blueprints/World/Items/BP_InspectActor Object Reference"))
  (return (cast `/Game/JttU/Blueprints/World/Items/BP_InspectActor` (`JCharacter.InspectActor` (`self.GetPlayerCharacter`)) :!pure true)))

(fn `LookAtSelectedActor`
  (params (SelectedActor :type "Actor Object Reference"))
  (bind (_returnvalue_roll _returnvalue_pitch _returnvalue_yaw) (`KismetMathLibrary.BreakRotator` (`KismetMathLibrary.FindLookAtRotation` (`self.K2_GetActorLocation` (`self.GetPlayerCharacter`)) (`self.K2_GetActorLocation` SelectedActor))))
  (`/Engine/EditorBlueprintResources/StandardMacros.IsValid` SelectedActor
    (:`Is Valid`
      (`self.K2_SetActorRotation` (`self.GetPlayerCharacter`) (`KismetMathLibrary.MakeRotator` 0.0 0.0 _returnvalue_yaw) true))))

(fn `MoveToUsable`
  (`JCharacter.MoveToUsableTimerStart` (`self.GetPlayerCharacter`)))

(fn `ShowActionsWidgetOnCursor`
  (params (SelectedActor :type "Actor Object Reference"))
  (bind (_locationx _locationy) (`self.GetMousePosition`))
  (`/Game/JttU/Blueprints/UI/Widgets/Actions/WBP_ActionsWidget.SetSelectedActor` (cast `/Game/JttU/Blueprints/UI/Widgets/Actions/WBP_ActionsWidget` (`JHUD.WBP_ActionsWidget` (`self.GetHUDGame`)) :!pure true) (`local.SelectedActor`))
  (`JHUD.ShowActionsWidget` (`self.GetHUDGame`) (`KismetMathLibrary.MakeVector2D` _locationx _locationy)))

(fn `ShowActionsWidgetOnObject`
  (params (SelectedActor :type "Actor Object Reference"))
  (bind _selectedactor (`local.SelectedActor`))
  (`/Game/JttU/Blueprints/UI/Widgets/Actions/WBP_ActionsWidget.SetSelectedActor` (cast `/Game/JttU/Blueprints/UI/Widgets/Actions/WBP_ActionsWidget` (`JHUD.WBP_ActionsWidget` (`self.GetHUDGame`)) :!pure true) _selectedactor)
  (`JHUD.ShowActionsWidget` (`self.GetHUDGame`) (`self.ProjectWorldLocationToScreen` (`JUsableActor.GetActionWidgetLocation` (cast `JUsableActor` _selectedactor :!pure true)))))

(fn `ToggleInventory`
  (locals (L_bDisableMovement :type Boolean))
  (bind _asbp_hud_game (`self.GetHUDGame`))
  (bind _wbp_inventory (`JHUD.WBP_Inventory` _asbp_hud_game))
  (if (`JHUD.IsInventoryOpen` _asbp_hud_game)
    (`JHUD.CloseWidget` _asbp_hud_game _wbp_inventory)
    (else
      (`JHUD.DisplayWidget` _asbp_hud_game _wbp_inventory)))
  (return))

(fn `UserConstructionScript`)